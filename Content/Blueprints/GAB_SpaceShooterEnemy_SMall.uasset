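; Small space shooter enemy that automatically fires projectiles on a repeating timer.
; After a random start delay of up to a second, it loops: spawn an enemy projectile at its own transform, play a sound, wait FiringRate.
; The sound plays at the world origin rather than at the enemy.
; Player health, score, ammo and weapon type getters are stubs returning zero.
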(event EventBeginPlay
  (Utilities|FlowControl|Delay (Math|Random|RandomFloatinRange 0.0 1.0))
  (Game|SpawnActorfromClass "/Game/Blueprints/GAB_SpaceShooterEnemyProj.GAB_SpaceShooterEnemyProj_C" (Transformation|GetActorTransform) "AdjustIfPossibleButDontSpawnIfColliding" 0 0 :!label _label)
  (Audio|PlaySoundatLocation "/Game/Audio/sepad_2__ad001_.sepad_2__ad001_" "0, 0, 0" "0, 0, 0" 1.0 1.0 0.0 0 0 0)
  (Utilities|FlowControl|Delay (Variables|Default|GetFiringRate))
  (goto _label))

(fn ConstructionScript)

(fn GetPlayerHealth
  (return 0))

(fn GetScore
  (return 0))

(fn GetAmmoCount
  (return 0))

(fn GetWeaponTYpe
  (return 0))